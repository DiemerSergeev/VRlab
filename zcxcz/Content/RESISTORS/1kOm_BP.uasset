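; Grabbable 1 kOm resistor that the player places into a fixed slot, setting the first resistor nominal on BP_Image_Streaming.
; Grabbing or clicking spawns a ghost placeholder at a hardcoded location.
; Overlapping a placeholder moves the resistor to that transform, releases it, then removes the ghost and returns the 16kOm and 11kOm resistors to their start positions.
; Dropping without overlap returns it to its start and removes the ghost.
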(event OnGrabbed(GrabComponent)
  (Variables|Default|SetOverlapped false)
  (bind _output_get (Variables|Default|SetSpawnLocation (Math|Transform|MakeTransform "115.000000,-59.000000,114.000000" "0, 0, 0" "1.000000,1.000000,1.000000")))
  (bind _returnvalue (Game|SpawnActorfromClass "/Game/RESISTORS/ResistorForPlace_Blueprint.ResistorForPlace_Blueprint_C" (Math|Transform|MakeTransform (.location _output_get) "0.000000,90.000000,0.000000" "1.000000,1.000000,1.000000") "Undefined" "MultiplyWithRoot" 0 0))
  (Variables|Default|SetGhost%20resistor _returnvalue)
  (Variables|Default|SetSpawn%20Transform (Transformation|GetActorTransform _returnvalue)))

(event OnDropped(GrabComponent)
  (if (not (Variables|Default|GetOverlapped))
    (Transformation|SetActorTransform (Class|KismetMathLibrary|TInterpto (Transformation|GetActorTransform) (Variables|Default|GetBeginPosition) 0.0 0.0))
    (Actor|DestroyActor (Variables|Default|GetGhost%20resistor))))

(event OnComponentBeginOverlap(Box)
  (params (OverlappedComponent :type Primitive%20Component%20Object%20Reference) (OtherActor :type Actor%20Object%20Reference) (OtherComp :type Primitive%20Component%20Object%20Reference) (OtherBodyIndex :type Integer) (bFromSweep :type Boolean) (SweepResult :type Hit%20Result%20Structure%20%28by%20ref%29))
  (Utilities|Casting|CastToResistorForPlace_Blueprint OtherActor)
  (Variables|Default|SetOverlapped true)
  (Utilities|FlowControl|Sequence
    (:then_0
      (Transformation|SetActorTransform (Class|KismetMathLibrary|TInterpto (Transformation|GetActorTransform) (Variables|Default|GetSpawn%20Transform) 0.0 0.0))
      (Default|TryRelease (Variables|Default|GetGrabComponent))
      (bind _returnvalue (Actor|GetActorOfClass "/Game/ImageStreaming/BP_Image_Streaming.BP_Image_Streaming_C"))
      (Variables|/Game/ImageStreaming/BP_Image_Streaming.BP_Image_Streaming_C|SetRESISTOR_NOMINAL1 _returnvalue "1"))
    (:then_1
      (if (Utilities|Operators|EqualEqual (.location (Variables|Default|GetSpawn%20Transform)) (Transformation|GetActorLocation) 0.001)
        (Utilities|FlowControl|Delay 0.1)
        (Actor|DestroyActor (Variables|Default|GetGhost%20resistor))
        (Utilities|FlowControl|Sequence
          (:then_0
            (bind _returnvalue_2 (Actor|GetActorOfClass "/Game/RESISTORS/16kOm.16kOm_C"))
            (Transformation|SetActorTransform _returnvalue_2 (Variables|/Game/RESISTORS/16kOm.16kOm_C|GetBeginPosition _returnvalue_2))
            (Development|PrintString "1kOm resistor added"))
          (:then_1
            (bind _returnvalue_3 (Actor|GetActorOfClass "/Game/RESISTORS/11kOm.11kOm_C"))
            (Transformation|SetActorTransform _returnvalue_3 (Variables|/Game/RESISTORS/11kOm.11kOm_C|GetBeginPosition _returnvalue_3))))))))

(event EventBeginPlay
  (Variables|Default|SetBeginPosition (Transformation|GetActorTransform)))

(event MouseInput|EventActorOnClicked
  (params (ButtonPressed :type Key%20Structure))
  (Variables|Default|SetOverlapped false)
  (bind _output_get (Variables|Default|SetSpawnLocation (Math|Transform|MakeTransform "115.000000,-59.000000,114.000000" "0, 0, 0" "1.000000,1.000000,1.000000")))
  (bind _returnvalue (Game|SpawnActorfromClass "/Game/RESISTORS/ResistorForPlace_Blueprint.ResistorForPlace_Blueprint_C" (Math|Transform|MakeTransform (.location _output_get) "0.000000,90.000000,0.000000" "1.000000,1.000000,1.000000") "Undefined" "MultiplyWithRoot" 0 0))
  (Variables|Default|SetGhost%20resistor _returnvalue)
  (Variables|Default|SetSpawn%20Transform (Transformation|GetActorTransform _returnvalue)))

(fn ConstructionScript)