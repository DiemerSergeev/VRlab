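; Virtual oscilloscope screen that drives remote lab hardware over HTTP and displays the captured image.
; Channel, scale and vertical-position events rebuild a command string, while other knob events only call wheel-selection actors.
; Single sends potentiometer and oscilloscope requests via VaRest, using timestamp IDs and fixed delays instead of response-driven sequencing.
; The downloaded BMP feeds a dynamic material on the Plane, then server entries are deleted and on-screen menus reset.
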(event Custom|OnOff
  (bind _plane (Variables|Default|GetPlane))
  ;[0 0 0] ON OFF
  (Utilities|FlowControl|FlipFlop
    (:A
      (Variables|Default|SetStatus true)
      (Rendering|Material|SetMaterial _plane 0 "/Game/Oscil/Meshes/Materials/no_chanel_Mat.no_chanel_Mat"))
    (:B
      (Variables|Default|SetStatus false)
      (Rendering|Material|SetMaterial _plane 0 "/Game/MATERIALS/Black.Black")))
  (bind _returnvalue (Actor|GetActorOfClass "/Game/BluePrint/Screen_menu_Blueprint.Screen_menu_Blueprint_C"))
  (Rendering|Material|SetMaterial (Variables|/Script/Engine.StaticMeshActor|GetStaticMeshComponent _returnvalue) 0 "/Game/Oscil/OscScreen/WORKED/Materials/Clear_screen.Clear_screen"))

(event Custom|Oscilllograph
  (params (Request :type Va%20Rest%20Request%20JSON%20Object%20Reference))
  ;[0 0 0] HTTP REQUEST
  (bind _returnvalue (Class|VaRestRequestJSON|GetResponseContentasString Request true))
  (Development|PrintString _returnvalue true true "(R=0.000000,G=0.660000,B=1.000000,A=1.000000)" 5.0))

(event Custom|CH1
  ;[0 0 0] CHANNEL
  (Variables|Default|SetIndex_CHANNELS "NewEnumerator13")
  (Variables|Default|SetCHANNEL (Utilities|Select :Index (Variables|Default|GetIndex_CHANNELS) :NewEnumerator13 (Variables|Default|GetCH1_) :NewEnumerator14 (Variables|Default|GetCH2_) :NewEnumerator15 (Variables|Default|GetCH3_) :NewEnumerator16 (Variables|Default|GetCH4_)))
  (Variables|Default|SetCHANNEL_STATUS true)
  ;[0 0 0] COMMAND STRING FOR OSCILLOSCOPE
  (Variables|Default|SetCommand_string (Utilities|Text|ToText(String) (Utilities|String|Append (Utilities|String|ToString(Text) (Utilities|Text|FormatText "CONFCHANNEL:[{CHANNEL};0][{SCALE_VERTICAL};{OFFSET_VERTICAL}];" (Variables|Default|GetCHANNEL) (Variables|Default|GetSCALE_Y) (Variables|Default|GetOFFSET_Y))) (Utilities|String|ToString(Text) (Utilities|Text|FormatText "CONFTIMEBASE:[{HORIZONTAL_SCALE}][0.000002000];" (stale Custom|ScaleXUpButton _output_get))))))
  (Utilities|FlowControl|Sequence
    (:then_0
      (if (not (Variables|Default|GetCHANNEL_STATUS))
        (Variables|Default|SetCHANNEL "1")))
    (:then_1
      (if (not (Variables|Default|GetSCALE_Y_STATUS))
        (Variables|Default|SetSCALE_Y "1")))
    (:then_2
      (if (not (Variables|Default|GetOFFSET_Y_STATUS))
        (Variables|Default|SetOFFSET_Y "0")))))

(event Custom|CH2
  ;[0 0 0] CHANNEL
  (Variables|Default|SetIndex_CHANNELS "NewEnumerator14")
  (Variables|Default|SetCHANNEL (Utilities|Select :Index (Variables|Default|GetIndex_CHANNELS) :NewEnumerator13 (Variables|Default|GetCH1_) :NewEnumerator14 (Variables|Default|GetCH2_) :NewEnumerator15 (Variables|Default|GetCH3_) :NewEnumerator16 (Variables|Default|GetCH4_)))
  (Variables|Default|SetCHANNEL_STATUS true)
  ;[0 0 0] COMMAND STRING FOR OSCILLOSCOPE
  (Variables|Default|SetCommand_string (Utilities|Text|ToText(String) (Utilities|String|Append (Utilities|String|ToString(Text) (Utilities|Text|FormatText "CONFCHANNEL:[{CHANNEL};0][{SCALE_VERTICAL};{OFFSET_VERTICAL}];" (Variables|Default|GetCHANNEL) (Variables|Default|GetSCALE_Y) (Variables|Default|GetOFFSET_Y))) (Utilities|String|ToString(Text) (Utilities|Text|FormatText "CONFTIMEBASE:[{HORIZONTAL_SCALE}][0.000002000];" (stale Custom|ScaleXUpButton _output_get))))))
  (Utilities|FlowControl|Sequence
    (:then_0
      (if (not (Variables|Default|GetCHANNEL_STATUS))
        (Variables|Default|SetCHANNEL "1")))
    (:then_1
      (if (not (Variables|Default|GetSCALE_Y_STATUS))
        (Variables|Default|SetSCALE_Y "1")))
    (:then_2
      (if (not (Variables|Default|GetOFFSET_Y_STATUS))
        (Variables|Default|SetOFFSET_Y "0")))))

(event Custom|CH3
  ;[0 0 0] CHANNEL
  (Variables|Default|SetIndex_CHANNELS "NewEnumerator15")
  (Variables|Default|SetCHANNEL (Utilities|Select :Index (Variables|Default|GetIndex_CHANNELS) :NewEnumerator13 (Variables|Default|GetCH1_) :NewEnumerator14 (Variables|Default|GetCH2_) :NewEnumerator15 (Variables|Default|GetCH3_) :NewEnumerator16 (Variables|Default|GetCH4_)))
  (Variables|Default|SetCHANNEL_STATUS true)
  ;[0 0 0] COMMAND STRING FOR OSCILLOSCOPE
  (Variables|Default|SetCommand_string (Utilities|Text|ToText(String) (Utilities|String|Append (Utilities|String|ToString(Text) (Utilities|Text|FormatText "CONFCHANNEL:[{CHANNEL};0][{SCALE_VERTICAL};{OFFSET_VERTICAL}];" (Variables|Default|GetCHANNEL) (Variables|Default|GetSCALE_Y) (Variables|Default|GetOFFSET_Y))) (Utilities|String|ToString(Text) (Utilities|Text|FormatText "CONFTIMEBASE:[{HORIZONTAL_SCALE}][0.000002000];" (stale Custom|ScaleXUpButton _output_get))))))
  (Utilities|FlowControl|Sequence
    (:then_0
      (if (not (Variables|Default|GetCHANNEL_STATUS))
        (Variables|Default|SetCHANNEL "1")))
    (:then_1
      (if (not (Variables|Default|GetSCALE_Y_STATUS))
        (Variables|Default|SetSCALE_Y "1")))
    (:then_2
      (if (not (Variables|Default|GetOFFSET_Y_STATUS))
        (Variables|Default|SetOFFSET_Y "0")))))

(event Custom|CH4
  ;[0 0 0] CHANNEL
  (Variables|Default|SetIndex_CHANNELS "NewEnumerator16")
  (Variables|Default|SetCHANNEL (Utilities|Select :Index (Variables|Default|GetIndex_CHANNELS) :NewEnumerator13 (Variables|Default|GetCH1_) :NewEnumerator14 (Variables|Default|GetCH2_) :NewEnumerator15 (Variables|Default|GetCH3_) :NewEnumerator16 (Variables|Default|GetCH4_)))
  (Variables|Default|SetCHANNEL_STATUS true)
  ;[0 0 0] COMMAND STRING FOR OSCILLOSCOPE
  (Variables|Default|SetCommand_string (Utilities|Text|ToText(String) (Utilities|String|Append (Utilities|String|ToString(Text) (Utilities|Text|FormatText "CONFCHANNEL:[{CHANNEL};0][{SCALE_VERTICAL};{OFFSET_VERTICAL}];" (Variables|Default|GetCHANNEL) (Variables|Default|GetSCALE_Y) (Variables|Default|GetOFFSET_Y))) (Utilities|String|ToString(Text) (Utilities|Text|FormatText "CONFTIMEBASE:[{HORIZONTAL_SCALE}][0.000002000];" (stale Custom|ScaleXUpButton _output_get))))))
  (Utilities|FlowControl|Sequence
    (:then_0
      (if (not (Variables|Default|GetCHANNEL_STATUS))
        (Variables|Default|SetCHANNEL "1")))
    (:then_1
      (if (not (Variables|Default|GetSCALE_Y_STATUS))
        (Variables|Default|SetSCALE_Y "1")))
    (:then_2
      (if (not (Variables|Default|GetOFFSET_Y_STATUS))
        (Variables|Default|SetOFFSET_Y "0")))))

(event Custom|Potentiometer
  (params (Request :type Va%20Rest%20Request%20JSON%20Object%20Reference))
  ;[0 0 0] HTTP REQUEST
  (bind _returnvalue (Class|VaRestRequestJSON|GetResponseContentasString Request true))
  (Development|PrintString _returnvalue true true "(R=0.000000,G=0.660000,B=1.000000,A=1.000000)" 5.0))

(event Custom|ScaleYUpButton
  (bind _y_scale_default (Variables|Default|GetY_Scale_default))
  ;[0 0 0] SCALE VERTICAL WIDGET
  (Variables|Default|Setindex_ScaleY "NewEnumerator0")
  (Variables|Default|SetSCALE_Y (Utilities|Select :Index (Variables|Default|Getindex_ScaleY) :NewEnumerator0 _y_scale_default :NewEnumerator1 (stale Custom|ScaleYRightButton _output_get) :NewEnumerator2 (stale Custom|ScaleYLeftButton _output_get) :NewEnumerator3 _y_scale_default))
  (Variables|Default|SetSCALE_Y_STATUS true)
  ;[0 0 0] COMMAND STRING FOR OSCILLOSCOPE
  (Variables|Default|SetCommand_string (Utilities|Text|ToText(String) (Utilities|String|Append (Utilities|String|ToString(Text) (Utilities|Text|FormatText "CONFCHANNEL:[{CHANNEL};0][{SCALE_VERTICAL};{OFFSET_VERTICAL}];" (Variables|Default|GetCHANNEL) (Variables|Default|GetSCALE_Y) (Variables|Default|GetOFFSET_Y))) (Utilities|String|ToString(Text) (Utilities|Text|FormatText "CONFTIMEBASE:[{HORIZONTAL_SCALE}][0.000002000];" (stale Custom|ScaleXUpButton _output_get))))))
  (Utilities|FlowControl|Sequence
    (:then_0
      (if (not (Variables|Default|GetCHANNEL_STATUS))
        (Variables|Default|SetCHANNEL "1")))
    (:then_1
      (if (not (Variables|Default|GetSCALE_Y_STATUS))
        (Variables|Default|SetSCALE_Y "1")))
    (:then_2
      (if (not (Variables|Default|GetOFFSET_Y_STATUS))
        (Variables|Default|SetOFFSET_Y "0")))))

(event Custom|ScaleYLeftButton
  ;[0 0 0] SCALE VERTICAL WIDGET
  (Variables|Default|Setindex_ScaleY "NewEnumerator2")
  (bind _output_get (Variables|Default|SetY_Scale_default (Utilities|String|ToString(Float) (/ (Math|Conversions|ToFloat(Integer) (Variables|Default|GetY_Scale_default)) 2.0))))
  (Variables|Default|SetSCALE_Y (Utilities|Select :Index (Variables|Default|Getindex_ScaleY) :NewEnumerator0 (Variables|Default|GetY_Scale_default) :NewEnumerator1 (stale Custom|ScaleYRightButton _output_get) :NewEnumerator2 _output_get :NewEnumerator3 (Variables|Default|GetY_Scale_default)))
  (Variables|Default|SetSCALE_Y_STATUS true)
  ;[0 0 0] COMMAND STRING FOR OSCILLOSCOPE
  (Variables|Default|SetCommand_string (Utilities|Text|ToText(String) (Utilities|String|Append (Utilities|String|ToString(Text) (Utilities|Text|FormatText "CONFCHANNEL:[{CHANNEL};0][{SCALE_VERTICAL};{OFFSET_VERTICAL}];" (Variables|Default|GetCHANNEL) (Variables|Default|GetSCALE_Y) (Variables|Default|GetOFFSET_Y))) (Utilities|String|ToString(Text) (Utilities|Text|FormatText "CONFTIMEBASE:[{HORIZONTAL_SCALE}][0.000002000];" (stale Custom|ScaleXUpButton _output_get))))))
  (Utilities|FlowControl|Sequence
    (:then_0
      (if (not (Variables|Default|GetCHANNEL_STATUS))
        (Variables|Default|SetCHANNEL "1")))
    (:then_1
      (if (not (Variables|Default|GetSCALE_Y_STATUS))
        (Variables|Default|SetSCALE_Y "1")))
    (:then_2
      (if (not (Variables|Default|GetOFFSET_Y_STATUS))
        (Variables|Default|SetOFFSET_Y "0")))))

(event Custom|PositionX2LeftButton
  ;[0 0 0] POSITION HORIZONTAL WIDGET
  (bind _returnvalue (Actor|GetActorOfClass "/Game/WheelSelection/WheelSelectionPositionX.WheelSelectionPositionX_C"))
  (Default|Select _returnvalue))

(event Custom|ScaleYRightButton
  ;[0 0 0] SCALE VERTICAL WIDGET
  (Variables|Default|Setindex_ScaleY "NewEnumerator1")
  (bind _output_get (Variables|Default|SetY_Scale_default (Utilities|String|ToString(Float) (* (Math|Conversions|ToFloat(Integer) (Variables|Default|GetY_Scale_default)) 2.0))))
  (Variables|Default|SetSCALE_Y (Utilities|Select :Index (Variables|Default|Getindex_ScaleY) :NewEnumerator0 (Variables|Default|GetY_Scale_default) :NewEnumerator1 _output_get :NewEnumerator2 (stale Custom|ScaleYLeftButton _output_get) :NewEnumerator3 (Variables|Default|GetY_Scale_default)))
  (Variables|Default|SetSCALE_Y_STATUS true)
  ;[0 0 0] COMMAND STRING FOR OSCILLOSCOPE
  (Variables|Default|SetCommand_string (Utilities|Text|ToText(String) (Utilities|String|Append (Utilities|String|ToString(Text) (Utilities|Text|FormatText "CONFCHANNEL:[{CHANNEL};0][{SCALE_VERTICAL};{OFFSET_VERTICAL}];" (Variables|Default|GetCHANNEL) (Variables|Default|GetSCALE_Y) (Variables|Default|GetOFFSET_Y))) (Utilities|String|ToString(Text) (Utilities|Text|FormatText "CONFTIMEBASE:[{HORIZONTAL_SCALE}][0.000002000];" (stale Custom|ScaleXUpButton _output_get))))))
  (Utilities|FlowControl|Sequence
    (:then_0
      (if (not (Variables|Default|GetCHANNEL_STATUS))
        (Variables|Default|SetCHANNEL "1")))
    (:then_1
      (if (not (Variables|Default|GetSCALE_Y_STATUS))
        (Variables|Default|SetSCALE_Y "1")))
    (:then_2
      (if (not (Variables|Default|GetOFFSET_Y_STATUS))
        (Variables|Default|SetOFFSET_Y "0")))))

(event Custom|PositionXLeftButton
  ;[0 0 0] POSITION HORIZONTAL WIDGET
  (bind _returnvalue (Actor|GetActorOfClass "/Game/WheelSelection/WheelSelectionPositionX.WheelSelectionPositionX_C"))
  (Default|Select _returnvalue))

(event Custom|PositionX2RightButton
  ;[0 0 0] POSITION HORIZONTAL WIDGET
  (bind _returnvalue (Actor|GetActorOfClass "/Game/WheelSelection/WheelSelectionPositionX.WheelSelectionPositionX_C"))
  (Default|Select _returnvalue))

(event Custom|Level2UpButton
  ;[0 0 0] LEVEL WIDGET
  (bind _returnvalue (Actor|GetActorOfClass "/Game/WheelSelection/WheelSelectionLevel.WheelSelectionLevel_C"))
  (Default|Select _returnvalue))

(event Custom|resistor%20nominal%20request%20delete
  (params (Request :type Va%20Rest%20Request%20JSON%20Object%20Reference))
  ;[0 0 0] HTTP REQUEST
  (bind _returnvalue (Class|VaRestRequestJSON|GetResponseContentasString Request true))
  (Development|PrintString _returnvalue true true "(R=0.000000,G=0.660000,B=1.000000,A=1.000000)" 5.0))

(event Custom|LevelUpButton
  ;[0 0 0] LEVEL WIDGET
  (bind _returnvalue (Actor|GetActorOfClass "/Game/WheelSelection/WheelSelectionLevel.WheelSelectionLevel_C"))
  (Default|Select _returnvalue))

(event Custom|Level2DownButton
  ;[0 0 0] LEVEL WIDGET
  (bind _returnvalue (Actor|GetActorOfClass "/Game/WheelSelection/WheelSelectionLevel.WheelSelectionLevel_C"))
  (Default|Select _returnvalue))

(event Custom|LevelDownButton
  ;[0 0 0] LEVEL WIDGET
  (bind _returnvalue (Actor|GetActorOfClass "/Game/WheelSelection/WheelSelectionLevel.WheelSelectionLevel_C"))
  (Default|Select _returnvalue))

(event Custom|LevelCenterButton
  ;[0 0 0] LEVEL WIDGET
  (bind _returnvalue (Actor|GetActorOfClass "/Game/WheelSelection/WheelSelectionLevel.WheelSelectionLevel_C"))
  (Default|Select _returnvalue))

(event Custom|PositionY2UpButton
  ;[0 0 0] POSITION VERTICAL WIDGET
  (Variables|Default|Setindex_OffsetY "NewEnumerator0")
  (Variables|Default|SetOFFSET_Y (Utilities|Select :Index (Variables|Default|Getindex_OffsetY) :NewEnumerator0 (Variables|Default|Get+3) :NewEnumerator1 (Variables|Default|Get+1) :NewEnumerator2 "0" :NewEnumerator3 (Variables|Default|Get-1) :NewEnumerator4 (Variables|Default|Get-3)))
  (Variables|Default|SetOFFSET_Y_STATUS true)
  ;[0 0 0] COMMAND STRING FOR OSCILLOSCOPE
  (Variables|Default|SetCommand_string (Utilities|Text|ToText(String) (Utilities|String|Append (Utilities|String|ToString(Text) (Utilities|Text|FormatText "CONFCHANNEL:[{CHANNEL};0][{SCALE_VERTICAL};{OFFSET_VERTICAL}];" (Variables|Default|GetCHANNEL) (Variables|Default|GetSCALE_Y) (Variables|Default|GetOFFSET_Y))) (Utilities|String|ToString(Text) (Utilities|Text|FormatText "CONFTIMEBASE:[{HORIZONTAL_SCALE}][0.000002000];" (stale Custom|ScaleXUpButton _output_get))))))
  (Utilities|FlowControl|Sequence
    (:then_0
      (if (not (Variables|Default|GetCHANNEL_STATUS))
        (Variables|Default|SetCHANNEL "1")))
    (:then_1
      (if (not (Variables|Default|GetSCALE_Y_STATUS))
        (Variables|Default|SetSCALE_Y "1")))
    (:then_2
      (if (not (Variables|Default|GetOFFSET_Y_STATUS))
        (Variables|Default|SetOFFSET_Y "0")))))

(event Custom|PositionYUpButton
  ;[0 0 0] POSITION VERTICAL WIDGET
  (Variables|Default|Setindex_OffsetY "NewEnumerator1")
  (Variables|Default|SetOFFSET_Y (Utilities|Select :Index (Variables|Default|Getindex_OffsetY) :NewEnumerator0 (Variables|Default|Get+3) :NewEnumerator1 (Variables|Default|Get+1) :NewEnumerator2 "0" :NewEnumerator3 (Variables|Default|Get-1) :NewEnumerator4 (Variables|Default|Get-3)))
  (Variables|Default|SetOFFSET_Y_STATUS true)
  ;[0 0 0] COMMAND STRING FOR OSCILLOSCOPE
  (Variables|Default|SetCommand_string (Utilities|Text|ToText(String) (Utilities|String|Append (Utilities|String|ToString(Text) (Utilities|Text|FormatText "CONFCHANNEL:[{CHANNEL};0][{SCALE_VERTICAL};{OFFSET_VERTICAL}];" (Variables|Default|GetCHANNEL) (Variables|Default|GetSCALE_Y) (Variables|Default|GetOFFSET_Y))) (Utilities|String|ToString(Text) (Utilities|Text|FormatText "CONFTIMEBASE:[{HORIZONTAL_SCALE}][0.000002000];" (stale Custom|ScaleXUpButton _output_get))))))
  (Utilities|FlowControl|Sequence
    (:then_0
      (if (not (Variables|Default|GetCHANNEL_STATUS))
        (Variables|Default|SetCHANNEL "1")))
    (:then_1
      (if (not (Variables|Default|GetSCALE_Y_STATUS))
        (Variables|Default|SetSCALE_Y "1")))
    (:then_2
      (if (not (Variables|Default|GetOFFSET_Y_STATUS))
        (Variables|Default|SetOFFSET_Y "0")))))

(event Custom|PositionYCenterButton
  ;[0 0 0] POSITION VERTICAL WIDGET
  (Variables|Default|Setindex_OffsetY "NewEnumerator2")
  (Variables|Default|SetOFFSET_Y (Utilities|Select :Index (Variables|Default|Getindex_OffsetY) :NewEnumerator0 (Variables|Default|Get+3) :NewEnumerator1 (Variables|Default|Get+1) :NewEnumerator2 "0" :NewEnumerator3 (Variables|Default|Get-1) :NewEnumerator4 (Variables|Default|Get-3)))
  (Variables|Default|SetOFFSET_Y_STATUS true)
  ;[0 0 0] COMMAND STRING FOR OSCILLOSCOPE
  (Variables|Default|SetCommand_string (Utilities|Text|ToText(String) (Utilities|String|Append (Utilities|String|ToString(Text) (Utilities|Text|FormatText "CONFCHANNEL:[{CHANNEL};0][{SCALE_VERTICAL};{OFFSET_VERTICAL}];" (Variables|Default|GetCHANNEL) (Variables|Default|GetSCALE_Y) (Variables|Default|GetOFFSET_Y))) (Utilities|String|ToString(Text) (Utilities|Text|FormatText "CONFTIMEBASE:[{HORIZONTAL_SCALE}][0.000002000];" (stale Custom|ScaleXUpButton _output_get))))))
  (Utilities|FlowControl|Sequence
    (:then_0
      (if (not (Variables|Default|GetCHANNEL_STATUS))
        (Variables|Default|SetCHANNEL "1")))
    (:then_1
      (if (not (Variables|Default|GetSCALE_Y_STATUS))
        (Variables|Default|SetSCALE_Y "1")))
    (:then_2
      (if (not (Variables|Default|GetOFFSET_Y_STATUS))
        (Variables|Default|SetOFFSET_Y "0")))))

(event Custom|PositionYDownButton
  ;[0 0 0] POSITION VERTICAL WIDGET
  (Variables|Default|Setindex_OffsetY "NewEnumerator3")
  (Variables|Default|SetOFFSET_Y (Utilities|Select :Index (Variables|Default|Getindex_OffsetY) :NewEnumerator0 (Variables|Default|Get+3) :NewEnumerator1 (Variables|Default|Get+1) :NewEnumerator2 "0" :NewEnumerator3 (Variables|Default|Get-1) :NewEnumerator4 (Variables|Default|Get-3)))
  (Variables|Default|SetOFFSET_Y_STATUS true)
  ;[0 0 0] COMMAND STRING FOR OSCILLOSCOPE
  (Variables|Default|SetCommand_string (Utilities|Text|ToText(String) (Utilities|String|Append (Utilities|String|ToString(Text) (Utilities|Text|FormatText "CONFCHANNEL:[{CHANNEL};0][{SCALE_VERTICAL};{OFFSET_VERTICAL}];" (Variables|Default|GetCHANNEL) (Variables|Default|GetSCALE_Y) (Variables|Default|GetOFFSET_Y))) (Utilities|String|ToString(Text) (Utilities|Text|FormatText "CONFTIMEBASE:[{HORIZONTAL_SCALE}][0.000002000];" (stale Custom|ScaleXUpButton _output_get))))))
  (Utilities|FlowControl|Sequence
    (:then_0
      (if (not (Variables|Default|GetCHANNEL_STATUS))
        (Variables|Default|SetCHANNEL "1")))
    (:then_1
      (if (not (Variables|Default|GetSCALE_Y_STATUS))
        (Variables|Default|SetSCALE_Y "1")))
    (:then_2
      (if (not (Variables|Default|GetOFFSET_Y_STATUS))
        (Variables|Default|SetOFFSET_Y "0")))))

(event Custom|PositionY2DownButton
  ;[0 0 0] POSITION VERTICAL WIDGET
  (Variables|Default|Setindex_OffsetY "NewEnumerator4")
  (Variables|Default|SetOFFSET_Y (Utilities|Select :Index (Variables|Default|Getindex_OffsetY) :NewEnumerator0 (Variables|Default|Get+3) :NewEnumerator1 (Variables|Default|Get+1) :NewEnumerator2 "0" :NewEnumerator3 (Variables|Default|Get-1) :NewEnumerator4 (Variables|Default|Get-3)))
  (Variables|Default|SetOFFSET_Y_STATUS true)
  ;[0 0 0] COMMAND STRING FOR OSCILLOSCOPE
  (Variables|Default|SetCommand_string (Utilities|Text|ToText(String) (Utilities|String|Append (Utilities|String|ToString(Text) (Utilities|Text|FormatText "CONFCHANNEL:[{CHANNEL};0][{SCALE_VERTICAL};{OFFSET_VERTICAL}];" (Variables|Default|GetCHANNEL) (Variables|Default|GetSCALE_Y) (Variables|Default|GetOFFSET_Y))) (Utilities|String|ToString(Text) (Utilities|Text|FormatText "CONFTIMEBASE:[{HORIZONTAL_SCALE}][0.000002000];" (stale Custom|ScaleXUpButton _output_get))))))
  (Utilities|FlowControl|Sequence
    (:then_0
      (if (not (Variables|Default|GetCHANNEL_STATUS))
        (Variables|Default|SetCHANNEL "1")))
    (:then_1
      (if (not (Variables|Default|GetSCALE_Y_STATUS))
        (Variables|Default|SetSCALE_Y "1")))
    (:then_2
      (if (not (Variables|Default|GetOFFSET_Y_STATUS))
        (Variables|Default|SetOFFSET_Y "0")))))

(event Custom|PositionXRightButton
  ;[0 0 0] POSITION HORIZONTAL WIDGET
  (bind _returnvalue (Actor|GetActorOfClass "/Game/WheelSelection/WheelSelectionPositionX.WheelSelectionPositionX_C"))
  (Default|Select _returnvalue))

(event Custom|Single
  (bind _returnvalue (Math|DateTime|Now))
  (bind _returnvalue_2 (Math|DateTime|Now))
  (bind _returnvalue_3 (|VaRestSubsystem))
  (bind _plane_material (Variables|Default|GetPlane%20Material))
  (bind (_year _month _day _hour _minute _second _millisecond) (Math|DateTime|BreakDateTime _returnvalue))
  (bind (_year_2 _month_2 _day_2 _hour_2 _minute_2 _second_2 _millisecond_2) (Math|DateTime|BreakDateTime _returnvalue_2))
  ;[0 0 0] REQUEST NAME
  (Variables|Default|Setreqnum_potentiometer (Utilities|String|Append (Utilities|String|ToString(Integer) _hour_2) (Utilities|String|ToString(Integer) _minute_2) (Utilities|String|ToString(Integer) _second_2) (Utilities|String|ToString(Integer) _millisecond_2)))
  (Variables|Default|Setreqnum (Utilities|String|Append (Utilities|String|ToString(Integer) _hour) (Utilities|String|ToString(Integer) _minute) (Utilities|String|ToString(Integer) _second) (Utilities|String|ToString(Integer) _millisecond)))
  ;[0 0 0] HTTP REQUEST
  (Class|VaRestSubsystem|CallURL _returnvalue_3 (Utilities|String|ToString(Text) (Utilities|Text|FormatText "http://31.134.128.28:8080/REST_GlassFish_HW_war/arduino/AddArduinoData?reqnum={reqnum}&userdata={userdata}" (Variables|Default|Getreqnum_potentiometer) (Utilities|Text|FormatText "ITOCW:[{adress}][0;{resistor1}];AI:[3][-1000];DI:[36][-1000];ITOCR:[44;1][-1000];EOC:ITOCW:[{adress}][128;{resistor2}];AI:[3][-1000];DI:[36][-1000];ITOCR:[44;1][-1000];EOC:" (Variables|Default|GetAdress) (Variables|Default|GetRESISTOR_NOMINAL1) (Variables|Default|GetRESISTOR_NOMINAL2)))) "GET" "x_www_form_urlencoded_url" 0 (delegate Custom|Potentiometer))
  (Development|PrintString "Success resistor nominal" true true "(R=0.000000,G=0.660000,B=1.000000,A=1.000000)" 5.0)
  (Utilities|FlowControl|Delay 0.5)
  (Class|VaRestSubsystem|CallURL _returnvalue_3 (Utilities|String|ToString(Text) (Utilities|Text|FormatText "http://31.134.128.28:8080/REST_GlassFish_HW_war/arduino/AddArduinoData?reqnum={reqnum}&userdata={userdata}" (Variables|Default|Getreqnum) (Utilities|String|Append (Utilities|String|ToString(Text) (Variables|Default|GetCommand_string)) (Utilities|String|ToString(Text) (Utilities|Text|FormatText "READWF:[{channel}][-997];GETPIC:[0][-997];EOC:" (Variables|Default|GetCHANNEL)))))) "GET" "x_www_form_urlencoded_url" 0 (delegate Custom|Oscilllograph))
  (Development|PrintString "Success oscillograph param" true true "(R=0.000000,G=0.660000,B=1.000000,A=1.000000)" 5.0)
  (Utilities|FlowControl|Delay 3.0)
  (bind _texture (|DownloadImage (Utilities|String|ToString(Text) (Utilities|Text|FormatText "http://31.134.128.28:8080/DownloadFileServlet/Download?filename={reqnum}.bmp" (Variables|Default|Getreqnum))))
    (:OnSuccess
      (Rendering|Material|SetTextureParameterValue _plane_material "Texture" _texture)
      (Rendering|Material|SetMaterial (Variables|Default|GetPlane) 0 _plane_material)
      (Class|VaRestSubsystem|CallURL (|VaRestSubsystem) (Utilities|String|ToString(Text) (Utilities|Text|FormatText "http://31.134.128.28:8080/REST_GlassFish_HW_war/arduino/RemoveArduinoEntry?reqnum={reqnum}" (Variables|Default|Getreqnum))) "GET" "x_www_form_urlencoded_url" 0 (delegate Custom|resistor%20nominal%20request%20delete))
      (Development|PrintString "Success! resistor nominal request deleted" true true "(R=0.000000,G=0.660000,B=1.000000,A=1.000000)" 5.0)
      (Class|VaRestSubsystem|CallURL (|VaRestSubsystem) (Utilities|String|ToString(Text) (Utilities|Text|FormatText "http://31.134.128.28:8080/REST_GlassFish_HW_war/arduino/RemoveArduinoEntry?reqnum={reqnum}" (Variables|Default|Getreqnum_potentiometer))) "GET" "x_www_form_urlencoded_url" 0 (delegate Custom|oscillograph%20request%20delete))
      (Development|PrintString "Success! oscillpgraph request deleted" true true "(R=0.000000,G=0.660000,B=1.000000,A=1.000000)" 5.0)
      ;[0 0 0] ADDITIONAL MENU OFF
      (bind _returnvalue_4 (Actor|GetActorOfClass "/Game/BluePrint/Screen_menu_Blueprint.Screen_menu_Blueprint_C"))
      (Rendering|Material|SetMaterial (Variables|/Script/Engine.StaticMeshActor|GetStaticMeshComponent _returnvalue_4) 0 "/Game/Oscil/OscScreen/WORKED/Materials/Clear_screen.Clear_screen")
      ;[0 0 0] RESET INDEX OF ADDITIONAL MENU
      (Utilities|FlowControl|Sequence
        (:then_0
          (bind _returnvalue_5 (Actor|GetActorOfClass "/Game/BluePrint/CH1_Blueprint.CH1_Blueprint_C"))
          (Variables|/Game/BluePrint/CH1_Blueprint.CH1_Blueprint_C|SetStatus _returnvalue_5 false))
        (:then_1
          (bind _returnvalue_6 (Actor|GetActorOfClass "/Game/BluePrint/oscillograph_Storage2_Blueprint.oscillograph_Storage2_Blueprint_C"))
          (Variables|/Game/BluePrint/oscillograph_Storage2_Blueprint.oscillograph_Storage2_Blueprint_C|SetStatus _returnvalue_6 false))
        (:then_2
          (bind _returnvalue_7 (Actor|GetActorOfClass "/Game/BluePrint/oscillograph_Acquire2_Blueprint.oscillograph_Acquire2_Blueprint_C"))
          (Variables|/Game/BluePrint/oscillograph_Acquire2_Blueprint.oscillograph_Acquire2_Blueprint_C|SetStatus _returnvalue_7 false))
        (:then_3
          (bind _returnvalue_8 (Actor|GetActorOfClass "/Game/BluePrint/oscillograph_Display2_Blueprint.oscillograph_Display2_Blueprint_C"))
          (Variables|/Game/BluePrint/oscillograph_Display2_Blueprint.oscillograph_Display2_Blueprint_C|SetStatus _returnvalue_8 false))
        (:then_4
          (bind _returnvalue_9 (Actor|GetActorOfClass "/Game/BluePrint/oscillograph_Utility2_Blueprint.oscillograph_Utility2_Blueprint_C"))
          (Variables|/Game/BluePrint/oscillograph_Utility2_Blueprint.oscillograph_Utility2_Blueprint_C|SetStatus _returnvalue_9 false))
        (:then_5
          (bind _returnvalue_10 (Actor|GetActorOfClass "/Game/BluePrint/oscillograph_Math2_Blueprint.oscillograph_Math2_Blueprint_C"))
          (Variables|/Game/BluePrint/oscillograph_Math2_Blueprint.oscillograph_Math2_Blueprint_C|SetStatus _returnvalue_10 false)
          (Variables|/Game/BluePrint/oscillograph_Math2_Blueprint.oscillograph_Math2_Blueprint_C|SetStatus_sheet_L _returnvalue_10 0)
          (Variables|/Game/BluePrint/oscillograph_Math2_Blueprint.oscillograph_Math2_Blueprint_C|SetStatus_sheet_R _returnvalue_10 0))
        (:then_6
          (bind _returnvalue_11 (Actor|GetActorOfClass "/Game/BluePrint/oscillograph_Ref2_Blueprint.oscillograph_Ref2_Blueprint_C"))
          (Variables|/Game/BluePrint/oscillograph_Ref2_Blueprint.oscillograph_Ref2_Blueprint_C|SetStatus _returnvalue_11 false))
        (:then_7
          (bind _returnvalue_12 (Actor|GetActorOfClass "/Game/BluePrint/oscillograph_Force2_Blueprint.oscillograph_Force2_Blueprint_C"))
          (Variables|/Game/BluePrint/oscillograph_Force2_Blueprint.oscillograph_Force2_Blueprint_C|SetStatus _returnvalue_12 false))
        (:then_8
          (bind _returnvalue_13 (Actor|GetActorOfClass "/Game/BluePrint/oscillograph_Help2_Blueprint.oscillograph_Help2_Blueprint_C"))
          (Variables|/Game/BluePrint/oscillograph_Help2_Blueprint.oscillograph_Help2_Blueprint_C|SetStatus _returnvalue_13 false))
        (:then_9
          (bind _returnvalue_14 (Actor|GetActorOfClass "/Game/BluePrint/oscillograph_S2_Blueprint.oscillograph_S2_Blueprint_C"))
          (Variables|/Game/BluePrint/oscillograph_S2_Blueprint.oscillograph_S2_Blueprint_C|SetStatus _returnvalue_14 false))
        (:then_10
          (bind _returnvalue_15 (Actor|GetActorOfClass "/Game/BluePrint/oscillograph_Menu4_Blueprint.oscillograph_Menu4_Blueprint_C"))
          (Variables|/Game/BluePrint/oscillograph_Menu4_Blueprint.oscillograph_Menu4_Blueprint_C|SetStatus _returnvalue_15 false))
        (:then_11
          (bind _returnvalue_16 (Actor|GetActorOfClass "/Game/BluePrint/oscillograph_Menu3_Blueprint.oscillograph_Menu3_Blueprint_C"))
          (Variables|/Game/BluePrint/oscillograph_Menu3_Blueprint.oscillograph_Menu3_Blueprint_C|SetStatus _returnvalue_16 false))
        (:then_12
          (bind _returnvalue_17 (Actor|GetActorOfClass "/Game/BluePrint/CH2_Blueprint.CH2_Blueprint_C"))
          (Variables|/Game/BluePrint/CH2_Blueprint.CH2_Blueprint_C|SetStatus _returnvalue_17 false))
        (:then_13
          (bind _returnvalue_18 (Actor|GetActorOfClass "/Game/BluePrint/CH3_Blueprint.CH3_Blueprint_C"))
          (Variables|/Game/BluePrint/CH3_Blueprint.CH3_Blueprint_C|SetStatus _returnvalue_18 false))
        (:then_14
          (bind _returnvalue_19 (Actor|GetActorOfClass "/Game/BluePrint/CH4_Blueprint.CH4_Blueprint_C"))
          (Variables|/Game/BluePrint/CH4_Blueprint.CH4_Blueprint_C|SetStatus _returnvalue_19 false))
        (:then_15
          (bind _returnvalue_20 (Actor|GetActorOfClass "/Game/BluePrint/oscillograph_Cursor2_Blueprint.oscillograph_Cursor2_Blueprint_C"))
          (Variables|/Game/BluePrint/oscillograph_Cursor2_Blueprint.oscillograph_Cursor2_Blueprint_C|SetStatus _returnvalue_20 false)
          (Variables|/Game/BluePrint/oscillograph_Cursor2_Blueprint.oscillograph_Cursor2_Blueprint_C|SetStatus_sheet _returnvalue_20 0))
        (:then_16
          (bind _returnvalue_21 (Actor|GetActorOfClass "/Game/BluePrint/oscillograph_Measure2_Blueprint.oscillograph_Measure2_Blueprint_C"))
          (Variables|/Game/BluePrint/oscillograph_Measure2_Blueprint.oscillograph_Measure2_Blueprint_C|SetStatus _returnvalue_21 false))))
    (:OnFail
      (Development|PrintString "Error resistor nominal" true true "(R=0.000000,G=0.660000,B=1.000000,A=1.000000)" 5.0))))

(event Custom|PositionXCenterButton
  ;[0 0 0] POSITION HORIZONTAL WIDGET
  (bind _returnvalue (Actor|GetActorOfClass "/Game/WheelSelection/WheelSelectionPositionX.WheelSelectionPositionX_C"))
  (Default|Select _returnvalue))

(event Custom|oscillograph%20request%20delete
  (params (Request :type Va%20Rest%20Request%20JSON%20Object%20Reference))
  ;[0 0 0] HTTP REQUEST
  (bind _returnvalue (Class|VaRestRequestJSON|GetResponseContentasString Request true))
  (Development|PrintString _returnvalue true true "(R=0.000000,G=0.660000,B=1.000000,A=1.000000)" 5.0))

(event Custom|IntensityWIdgetUpButton
  ;[0 0 0] INTENSITY WIDGET
  (bind _returnvalue (Actor|GetActorOfClass "/Game/WheelSelection/WheelSelectionIntensity.WheelSelectionIntensity_C"))
  (Default|Select _returnvalue))

(event Custom|IntensityWidgetRIghtButton
  ;[0 0 0] INTENSITY WIDGET
  (bind _returnvalue (Actor|GetActorOfClass "/Game/WheelSelection/WheelSelectionIntensity.WheelSelectionIntensity_C"))
  (Default|Select _returnvalue))

(event Custom|IntensityWidgetLeftButton
  ;[0 0 0] INTENSITY WIDGET
  (bind _returnvalue (Actor|GetActorOfClass "/Game/WheelSelection/WheelSelectionIntensity.WheelSelectionIntensity_C"))
  (Default|Select _returnvalue))

(event Custom|IntensityWidgetCenterButton
  ;[0 0 0] INTENSITY WIDGET
  (bind _returnvalue (Actor|GetActorOfClass "/Game/WheelSelection/WheelSelectionIntensity.WheelSelectionIntensity_C"))
  (Default|Select _returnvalue))

(event Custom|ScaleYCenterButton
  (bind _y_scale_default (Variables|Default|GetY_Scale_default))
  ;[0 0 0] SCALE VERTICAL WIDGET
  (Variables|Default|Setindex_ScaleY "NewEnumerator3")
  (Variables|Default|SetSCALE_Y (Utilities|Select :Index (Variables|Default|Getindex_ScaleY) :NewEnumerator0 _y_scale_default :NewEnumerator1 (stale Custom|ScaleYRightButton _output_get) :NewEnumerator2 (stale Custom|ScaleYLeftButton _output_get) :NewEnumerator3 _y_scale_default))
  (Variables|Default|SetSCALE_Y_STATUS true)
  ;[0 0 0] COMMAND STRING FOR OSCILLOSCOPE
  (Variables|Default|SetCommand_string (Utilities|Text|ToText(String) (Utilities|String|Append (Utilities|String|ToString(Text) (Utilities|Text|FormatText "CONFCHANNEL:[{CHANNEL};0][{SCALE_VERTICAL};{OFFSET_VERTICAL}];" (Variables|Default|GetCHANNEL) (Variables|Default|GetSCALE_Y) (Variables|Default|GetOFFSET_Y))) (Utilities|String|ToString(Text) (Utilities|Text|FormatText "CONFTIMEBASE:[{HORIZONTAL_SCALE}][0.000002000];" (stale Custom|ScaleXUpButton _output_get))))))
  (Utilities|FlowControl|Sequence
    (:then_0
      (if (not (Variables|Default|GetCHANNEL_STATUS))
        (Variables|Default|SetCHANNEL "1")))
    (:then_1
      (if (not (Variables|Default|GetSCALE_Y_STATUS))
        (Variables|Default|SetSCALE_Y "1")))
    (:then_2
      (if (not (Variables|Default|GetOFFSET_Y_STATUS))
        (Variables|Default|SetOFFSET_Y "0")))))

(event Custom|ScaleXUpButton
  (bind _h_scale_default (Variables|Default|GetH_Scale_default))
  ;[0 0 0] HORIZONTAL SCALE
  (Variables|Default|Setindex_ScaleX "NewEnumerator0")
  (bind _output_get (Variables|Default|SetSCALE_X (Utilities|Select :Index (Variables|Default|Getindex_ScaleX) :NewEnumerator0 _h_scale_default :NewEnumerator1 (stale Custom|ScaleXRightButton _output_get) :NewEnumerator2 (stale Custom|ScaleXLeftButton _output_get) :NewEnumerator3 _h_scale_default)))
  ;[0 0 0] COMMAND STRING FOR OSCILLOSCOPE
  (Variables|Default|SetCommand_string (Utilities|Text|ToText(String) (Utilities|String|Append (Utilities|String|ToString(Text) (Utilities|Text|FormatText "CONFCHANNEL:[{CHANNEL};0][{SCALE_VERTICAL};{OFFSET_VERTICAL}];" (Variables|Default|GetCHANNEL) (Variables|Default|GetSCALE_Y) (Variables|Default|GetOFFSET_Y))) (Utilities|String|ToString(Text) (Utilities|Text|FormatText "CONFTIMEBASE:[{HORIZONTAL_SCALE}][0.000002000];" _output_get)))))
  (Utilities|FlowControl|Sequence
    (:then_0
      (if (not (Variables|Default|GetCHANNEL_STATUS))
        (Variables|Default|SetCHANNEL "1")))
    (:then_1
      (if (not (Variables|Default|GetSCALE_Y_STATUS))
        (Variables|Default|SetSCALE_Y "1")))
    (:then_2
      (if (not (Variables|Default|GetOFFSET_Y_STATUS))
        (Variables|Default|SetOFFSET_Y "0")))))

(event Custom|ScaleXCenterButton
  (bind _h_scale_default (Variables|Default|GetH_Scale_default))
  ;[0 0 0] HORIZONTAL SCALE
  (Variables|Default|Setindex_ScaleX "NewEnumerator3")
  (bind _output_get (Variables|Default|SetSCALE_X (Utilities|Select :Index (Variables|Default|Getindex_ScaleX) :NewEnumerator0 _h_scale_default :NewEnumerator1 (stale Custom|ScaleXRightButton _output_get) :NewEnumerator2 (stale Custom|ScaleXLeftButton _output_get) :NewEnumerator3 _h_scale_default)))
  ;[0 0 0] COMMAND STRING FOR OSCILLOSCOPE
  (Variables|Default|SetCommand_string (Utilities|Text|ToText(String) (Utilities|String|Append (Utilities|String|ToString(Text) (Utilities|Text|FormatText "CONFCHANNEL:[{CHANNEL};0][{SCALE_VERTICAL};{OFFSET_VERTICAL}];" (Variables|Default|GetCHANNEL) (Variables|Default|GetSCALE_Y) (Variables|Default|GetOFFSET_Y))) (Utilities|String|ToString(Text) (Utilities|Text|FormatText "CONFTIMEBASE:[{HORIZONTAL_SCALE}][0.000002000];" _output_get)))))
  (Utilities|FlowControl|Sequence
    (:then_0
      (if (not (Variables|Default|GetCHANNEL_STATUS))
        (Variables|Default|SetCHANNEL "1")))
    (:then_1
      (if (not (Variables|Default|GetSCALE_Y_STATUS))
        (Variables|Default|SetSCALE_Y "1")))
    (:then_2
      (if (not (Variables|Default|GetOFFSET_Y_STATUS))
        (Variables|Default|SetOFFSET_Y "0")))))

(event Custom|ScaleXRightButton
  ;[0 0 0] HORIZONTAL SCALE
  (Variables|Default|Setindex_ScaleX "NewEnumerator1")
  (bind _output_get (Variables|Default|SetH_Scale_default (Utilities|String|ToString(Float) (* (Math|Conversions|ToFloat(Integer) (Variables|Default|GetH_Scale_default)) 2.0))))
  (bind _output_get_2 (Variables|Default|SetSCALE_X (Utilities|Select :Index (Variables|Default|Getindex_ScaleX) :NewEnumerator0 (Variables|Default|GetH_Scale_default) :NewEnumerator1 _output_get :NewEnumerator2 (stale Custom|ScaleXLeftButton _output_get) :NewEnumerator3 (Variables|Default|GetH_Scale_default))))
  ;[0 0 0] COMMAND STRING FOR OSCILLOSCOPE
  (Variables|Default|SetCommand_string (Utilities|Text|ToText(String) (Utilities|String|Append (Utilities|String|ToString(Text) (Utilities|Text|FormatText "CONFCHANNEL:[{CHANNEL};0][{SCALE_VERTICAL};{OFFSET_VERTICAL}];" (Variables|Default|GetCHANNEL) (Variables|Default|GetSCALE_Y) (Variables|Default|GetOFFSET_Y))) (Utilities|String|ToString(Text) (Utilities|Text|FormatText "CONFTIMEBASE:[{HORIZONTAL_SCALE}][0.000002000];" _output_get_2)))))
  (Utilities|FlowControl|Sequence
    (:then_0
      (if (not (Variables|Default|GetCHANNEL_STATUS))
        (Variables|Default|SetCHANNEL "1")))
    (:then_1
      (if (not (Variables|Default|GetSCALE_Y_STATUS))
        (Variables|Default|SetSCALE_Y "1")))
    (:then_2
      (if (not (Variables|Default|GetOFFSET_Y_STATUS))
        (Variables|Default|SetOFFSET_Y "0")))))

(event Custom|ScaleXLeftButton
  ;[0 0 0] HORIZONTAL SCALE
  (Variables|Default|Setindex_ScaleX "NewEnumerator2")
  (bind _output_get (Variables|Default|SetH_Scale_default (Utilities|String|ToString(Float) (/ (Math|Conversions|ToFloat(Integer) (Variables|Default|GetH_Scale_default)) 2.0))))
  (bind _output_get_2 (Variables|Default|SetSCALE_X (Utilities|Select :Index (Variables|Default|Getindex_ScaleX) :NewEnumerator0 (Variables|Default|GetH_Scale_default) :NewEnumerator1 (stale Custom|ScaleXRightButton _output_get) :NewEnumerator2 _output_get :NewEnumerator3 (Variables|Default|GetH_Scale_default))))
  ;[0 0 0] COMMAND STRING FOR OSCILLOSCOPE
  (Variables|Default|SetCommand_string (Utilities|Text|ToText(String) (Utilities|String|Append (Utilities|String|ToString(Text) (Utilities|Text|FormatText "CONFCHANNEL:[{CHANNEL};0][{SCALE_VERTICAL};{OFFSET_VERTICAL}];" (Variables|Default|GetCHANNEL) (Variables|Default|GetSCALE_Y) (Variables|Default|GetOFFSET_Y))) (Utilities|String|ToString(Text) (Utilities|Text|FormatText "CONFTIMEBASE:[{HORIZONTAL_SCALE}][0.000002000];" _output_get_2)))))
  (Utilities|FlowControl|Sequence
    (:then_0
      (if (not (Variables|Default|GetCHANNEL_STATUS))
        (Variables|Default|SetCHANNEL "1")))
    (:then_1
      (if (not (Variables|Default|GetSCALE_Y_STATUS))
        (Variables|Default|SetSCALE_Y "1")))
    (:then_2
      (if (not (Variables|Default|GetOFFSET_Y_STATUS))
        (Variables|Default|SetOFFSET_Y "0")))))

(fn ConstructionScript
  (bind _returnvalue (Rendering|Material|CreateDynamicMaterialInstance (Variables|Default|GetPlane) 0 "/Game/ImageStreaming/MM_Image_Streaming.MM_Image_Streaming" "None" :!class /Script/Engine.PrimitiveComponent))
  (Variables|Default|SetPlane%20Material _returnvalue))