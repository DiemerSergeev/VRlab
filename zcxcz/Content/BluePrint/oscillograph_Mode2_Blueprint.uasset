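; Oscilloscope Mode 2 control that cycles the lit indicator through Auto, Normal and Single each time it is grabbed.
; It responds only while the Status flag on BP_Image_Streaming is true.
; A looping, ordered MultiGate finds the three indicator actors by class and swaps their materials, giving the active one a glowing LED and the other two the plain LED material.
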(event OnGrabbed(GrabComponent)
  (bind _returnvalue (Actor|GetActorOfClass "/Game/ImageStreaming/BP_Image_Streaming.BP_Image_Streaming_C"))
  (if (Variables|/Game/ImageStreaming/BP_Image_Streaming.BP_Image_Streaming_C|GetStatus _returnvalue)
    (Utilities|FlowControl|MultiGate false true -1
      (:Out%200
        (bind _returnvalue_2 (Actor|GetActorOfClass "/Game/BluePrint/oscillograph_Single_mode2_Blueprint.oscillograph_Single_mode2_Blueprint_C"))
        (bind _returnvalue_3 (Actor|GetActorOfClass "/Game/BluePrint/oscillograph_Normal2_Blueprint.oscillograph_Normal2_Blueprint_C"))
        (Rendering|Material|SetMaterial (Variables|/Script/Engine.StaticMeshActor|GetStaticMeshComponent _returnvalue_2) 0 "/Game/Oscil/Meshes/Materials/Material_leds.Material_leds")
        (bind _returnvalue_4 (Actor|GetActorOfClass "/Game/Oscil/Meshes/BP/oscillograph_Auto_BP.oscillograph_Auto_BP_C"))
        (Rendering|Material|SetMaterial (Variables|/Script/Engine.StaticMeshActor|GetStaticMeshComponent _returnvalue_4) 0 "/Game/Oscil/Meshes/Materials/Glow_LED_Inst.Glow_LED_Inst"))
      (:Out%201
        (bind _returnvalue_5 (Actor|GetActorOfClass "/Game/BluePrint/oscillograph_Single_mode2_Blueprint.oscillograph_Single_mode2_Blueprint_C"))
        (bind _returnvalue_6 (Actor|GetActorOfClass "/Game/Oscil/Meshes/BP/oscillograph_Auto_BP.oscillograph_Auto_BP_C"))
        (Rendering|Material|SetMaterial (Variables|/Script/Engine.StaticMeshActor|GetStaticMeshComponent _returnvalue_5) 0 "/Game/Oscil/Meshes/Materials/Material_leds.Material_leds")
        (bind _returnvalue_7 (Actor|GetActorOfClass "/Game/BluePrint/oscillograph_Normal2_Blueprint.oscillograph_Normal2_Blueprint_C"))
        (Rendering|Material|SetMaterial (Variables|/Script/Engine.StaticMeshActor|GetStaticMeshComponent _returnvalue_7) 0 "/Game/Oscil/Meshes/Materials/Glow_LED_Inst.Glow_LED_Inst"))
      (:Out%202
        (bind _returnvalue_8 (Actor|GetActorOfClass "/Game/Oscil/Meshes/BP/oscillograph_Auto_BP.oscillograph_Auto_BP_C"))
        (bind _returnvalue_9 (Actor|GetActorOfClass "/Game/BluePrint/oscillograph_Normal2_Blueprint.oscillograph_Normal2_Blueprint_C"))
        (Rendering|Material|SetMaterial (Variables|/Script/Engine.StaticMeshActor|GetStaticMeshComponent _returnvalue_9) 0 "/Game/Oscil/Meshes/Materials/Material_leds.Material_leds")
        (bind _returnvalue_10 (Actor|GetActorOfClass "/Game/BluePrint/oscillograph_Single_mode2_Blueprint.oscillograph_Single_mode2_Blueprint_C"))
        (Rendering|Material|SetMaterial (Variables|/Script/Engine.StaticMeshActor|GetStaticMeshComponent _returnvalue_10) 0 "/Game/Oscil/Meshes/Materials/Glow_LED_Inst.Glow_LED_Inst")))))

(fn ConstructionScript)