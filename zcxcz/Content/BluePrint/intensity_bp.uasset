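; Grabbable VR actor that opens and confirms an intensity selection wheel when BP_Image_Streaming's Status is true.
; Each qualifying grab drives a FlipFlop: the first spawns WheelSelectionIntensity at the VRPawn's right motion controller using only its yaw, the next calls Select on that wheel if still valid.
; The streaming actor and pawn are found with GetActorOfClass, and placement uses the right controller regardless of the grabbing hand.
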(event OnGrabbed(GrabComponent)
  (bind _returnvalue (Actor|GetActorOfClass "/Game/ImageStreaming/BP_Image_Streaming.BP_Image_Streaming_C"))
  (if (Variables|/Game/ImageStreaming/BP_Image_Streaming.BP_Image_Streaming_C|GetStatus _returnvalue)
    (bind _returnvalue_2 (Actor|GetActorOfClass "/Game/VRTemplate/Blueprints/VRPawn.VRPawn_C"))
    (Utilities|FlowControl|FlipFlop
      (:A
        (bind _returnvalue_3 (Game|SpawnActorfromClass "/Game/WheelSelection/WheelSelectionIntensity.WheelSelectionIntensity_C" (Math|Transform|MakeTransform (.location (Transformation|GetWorldTransform (Variables|/Game/VRTemplate/Blueprints/VRPawn.VRPawn_C|GetMotionControllerRight _returnvalue_2))) (Math|Rotator|MakeRotator 0.0 0.0 (.yaw (.rotation (Transformation|GetWorldTransform (Variables|/Game/VRTemplate/Blueprints/VRPawn.VRPawn_C|GetMotionControllerRight _returnvalue_2))))) "1.000000,1.000000,1.000000") "Undefined" "MultiplyWithRoot" 0 0 0))
        (Variables|Default|SetRightHandle _returnvalue_3))
      (:B
        (bind _righthandle (Variables|Default|GetRightHandle)
          (:then
            (Default|Select _righthandle))
          (:else))))))

(fn ConstructionScript)