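; Fourth right-menu button in VR that, when grabbed, drives the scale selection wheel for oscillograph measurement 1.
; It acts only while both BP_Image_Streaming and Oscillograph_Measure2_Blueprint have Status set.
; A FlipFlop alternates between spawning WheelSelectionScaleMeasure1 at the VRPawn's right motion controller, yaw-aligned and given that controller, and calling Select on RightHandle if valid.
; The spawn branch sets RightHandle to None rather than the spawned wheel.
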(event OnGrabbed(GrabComponent)
  (bind _returnvalue (Actor|GetActorOfClass "/Game/ImageStreaming/BP_Image_Streaming.BP_Image_Streaming_C"))
  (if (Variables|/Game/ImageStreaming/BP_Image_Streaming.BP_Image_Streaming_C|GetStatus _returnvalue)
    (bind _returnvalue_2 (Actor|GetActorOfClass "/Game/BluePrint/oscillograph_Measure2_Blueprint.oscillograph_Measure2_Blueprint_C"))
    (if (Variables|/Game/BluePrint/oscillograph_Measure2_Blueprint.oscillograph_Measure2_Blueprint_C|GetStatus _returnvalue_2)
      (bind _returnvalue_3 (Actor|GetActorOfClass "/Game/VRTemplate/Blueprints/VRPawn.VRPawn_C"))
      (Utilities|FlowControl|FlipFlop
        (:A
          (Game|SpawnActorfromClass "/Game/WheelSelection/WheelSelectionScaleMeasure1.WheelSelectionScaleMeasure1_C" (Math|Transform|MakeTransform (.location (Transformation|GetWorldTransform (Variables|/Game/VRTemplate/Blueprints/VRPawn.VRPawn_C|GetMotionControllerRight _returnvalue_3))) (Math|Rotator|MakeRotator 0.0 0.0 (.yaw (.rotation (Transformation|GetWorldTransform (Variables|/Game/VRTemplate/Blueprints/VRPawn.VRPawn_C|GetMotionControllerRight _returnvalue_3))))) "1.000000,1.000000,1.000000") "Undefined" "MultiplyWithRoot" 0 (Variables|/Game/VRTemplate/Blueprints/VRPawn.VRPawn_C|GetMotionControllerRight _returnvalue_3) 0)
          (Variables|Default|SetRightHandle 0))
        (:B
          (bind _righthandle (Variables|Default|GetRightHandle)
            (:then
              (Default|Select _righthandle))
            (:else)))))))

(fn ConstructionScript)