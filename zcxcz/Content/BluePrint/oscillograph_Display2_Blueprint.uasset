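; Display button of a virtual oscilloscope that opens the display menu on the instrument's screen when grabbed.
; If BP_Image_Streaming's Status is on, the grab event applies the display material to the screen menu mesh and sets its own Status.
; A Sequence then clears Status on the other menu and channel buttons, also resetting Math and Cursor sheet states.
; Each actor is found at grab time with GetActorOfClass.
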(event OnGrabbed(GrabComponent)
  (bind _returnvalue (Actor|GetActorOfClass "/Game/ImageStreaming/BP_Image_Streaming.BP_Image_Streaming_C"))
  (if (Variables|/Game/ImageStreaming/BP_Image_Streaming.BP_Image_Streaming_C|GetStatus _returnvalue)
    (bind _returnvalue_2 (Actor|GetActorOfClass "/Game/BluePrint/Screen_menu_Blueprint.Screen_menu_Blueprint_C"))
    (Rendering|Material|SetMaterial (Variables|/Script/Engine.StaticMeshActor|GetStaticMeshComponent _returnvalue_2) 0 "/Game/Oscil/OscScreen/WORKED/Materials/DISPLAY_1_Mat.DISPLAY_1_Mat")
    (Variables|Default|SetStatus true)
    (Utilities|FlowControl|Sequence
      (:then_0
        (bind _returnvalue_3 (Actor|GetActorOfClass "/Game/BluePrint/oscillograph_Measure2_Blueprint.oscillograph_Measure2_Blueprint_C"))
        (Variables|/Game/BluePrint/oscillograph_Measure2_Blueprint.oscillograph_Measure2_Blueprint_C|SetStatus _returnvalue_3 false))
      (:then_1
        (bind _returnvalue_4 (Actor|GetActorOfClass "/Game/BluePrint/oscillograph_Storage2_Blueprint.oscillograph_Storage2_Blueprint_C"))
        (Variables|/Game/BluePrint/oscillograph_Storage2_Blueprint.oscillograph_Storage2_Blueprint_C|SetStatus _returnvalue_4 false))
      (:then_2
        (bind _returnvalue_5 (Actor|GetActorOfClass "/Game/BluePrint/oscillograph_Acquire2_Blueprint.oscillograph_Acquire2_Blueprint_C"))
        (Variables|/Game/BluePrint/oscillograph_Acquire2_Blueprint.oscillograph_Acquire2_Blueprint_C|SetStatus _returnvalue_5 false))
      (:then_3
        (bind _returnvalue_6 (Actor|GetActorOfClass "/Game/BluePrint/CH1_Blueprint.CH1_Blueprint_C"))
        (Variables|/Game/BluePrint/CH1_Blueprint.CH1_Blueprint_C|SetStatus _returnvalue_6 false))
      (:then_4
        (bind _returnvalue_7 (Actor|GetActorOfClass "/Game/BluePrint/oscillograph_Utility2_Blueprint.oscillograph_Utility2_Blueprint_C"))
        (Variables|/Game/BluePrint/oscillograph_Utility2_Blueprint.oscillograph_Utility2_Blueprint_C|SetStatus _returnvalue_7 false))
      (:then_5
        (bind _returnvalue_8 (Actor|GetActorOfClass "/Game/BluePrint/oscillograph_Math2_Blueprint.oscillograph_Math2_Blueprint_C"))
        (Variables|/Game/BluePrint/oscillograph_Math2_Blueprint.oscillograph_Math2_Blueprint_C|SetStatus _returnvalue_8 false)
        (Variables|/Game/BluePrint/oscillograph_Math2_Blueprint.oscillograph_Math2_Blueprint_C|SetStatus_sheet_L _returnvalue_8 0)
        (Variables|/Game/BluePrint/oscillograph_Math2_Blueprint.oscillograph_Math2_Blueprint_C|SetStatus_sheet_R _returnvalue_8 0))
      (:then_6
        (bind _returnvalue_9 (Actor|GetActorOfClass "/Game/BluePrint/oscillograph_Ref2_Blueprint.oscillograph_Ref2_Blueprint_C"))
        (Variables|/Game/BluePrint/oscillograph_Ref2_Blueprint.oscillograph_Ref2_Blueprint_C|SetStatus _returnvalue_9 false))
      (:then_7
        (bind _returnvalue_10 (Actor|GetActorOfClass "/Game/BluePrint/oscillograph_Force2_Blueprint.oscillograph_Force2_Blueprint_C"))
        (Variables|/Game/BluePrint/oscillograph_Force2_Blueprint.oscillograph_Force2_Blueprint_C|SetStatus _returnvalue_10 false))
      (:then_8
        (bind _returnvalue_11 (Actor|GetActorOfClass "/Game/BluePrint/oscillograph_Help2_Blueprint.oscillograph_Help2_Blueprint_C"))
        (Variables|/Game/BluePrint/oscillograph_Help2_Blueprint.oscillograph_Help2_Blueprint_C|SetStatus _returnvalue_11 false))
      (:then_9
        (bind _returnvalue_12 (Actor|GetActorOfClass "/Game/BluePrint/oscillograph_S2_Blueprint.oscillograph_S2_Blueprint_C"))
        (Variables|/Game/BluePrint/oscillograph_S2_Blueprint.oscillograph_S2_Blueprint_C|SetStatus _returnvalue_12 false))
      (:then_10
        (bind _returnvalue_13 (Actor|GetActorOfClass "/Game/BluePrint/oscillograph_Menu4_Blueprint.oscillograph_Menu4_Blueprint_C"))
        (Variables|/Game/BluePrint/oscillograph_Menu4_Blueprint.oscillograph_Menu4_Blueprint_C|SetStatus _returnvalue_13 false))
      (:then_11
        (bind _returnvalue_14 (Actor|GetActorOfClass "/Game/BluePrint/oscillograph_Menu3_Blueprint.oscillograph_Menu3_Blueprint_C"))
        (Variables|/Game/BluePrint/oscillograph_Menu3_Blueprint.oscillograph_Menu3_Blueprint_C|SetStatus _returnvalue_14 false))
      (:then_12
        (bind _returnvalue_15 (Actor|GetActorOfClass "/Game/BluePrint/CH2_Blueprint.CH2_Blueprint_C"))
        (Variables|/Game/BluePrint/CH2_Blueprint.CH2_Blueprint_C|SetStatus _returnvalue_15 false))
      (:then_13
        (bind _returnvalue_16 (Actor|GetActorOfClass "/Game/BluePrint/CH3_Blueprint.CH3_Blueprint_C"))
        (Variables|/Game/BluePrint/CH3_Blueprint.CH3_Blueprint_C|SetStatus _returnvalue_16 false))
      (:then_14
        (bind _returnvalue_17 (Actor|GetActorOfClass "/Game/BluePrint/CH4_Blueprint.CH4_Blueprint_C"))
        (Variables|/Game/BluePrint/CH4_Blueprint.CH4_Blueprint_C|SetStatus _returnvalue_17 false))
      (:then_15
        (bind _returnvalue_18 (Actor|GetActorOfClass "/Game/BluePrint/oscillograph_Cursor2_Blueprint.oscillograph_Cursor2_Blueprint_C"))
        (Variables|/Game/BluePrint/oscillograph_Cursor2_Blueprint.oscillograph_Cursor2_Blueprint_C|SetStatus _returnvalue_18 false)
        (Variables|/Game/BluePrint/oscillograph_Cursor2_Blueprint.oscillograph_Cursor2_Blueprint_C|SetStatus_sheet _returnvalue_18 0)))))

(fn ConstructionScript)