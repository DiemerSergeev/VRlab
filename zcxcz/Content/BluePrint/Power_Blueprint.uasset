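; Grabbable power button for an oscilloscope, toggling the instrument on and off.
; Each grab flip-flops: on lights the Single-mode and CH1 indicators, off resets mode LEDs, channels, Run/Stop and menu screen, and both call OnOff on BP_Image_Streaming.
; A Delay on Tick alternates the Run/Stop glow about every five seconds while the streamer's Status is true.
; Other parts are found by GetActorOfClass.
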(event OnGrabbed(GrabComponent)
  (bind _staticmeshcomponent (Variables|Debug|GetStaticMeshComponent))
  (Utilities|FlowControl|FlipFlop
    (:A
      (Rendering|Material|SetMaterial _staticmeshcomponent 0 "/Game/Oscil/Meshes/Materials/Material_002.Material_002")
      (bind _returnvalue (Actor|GetActorOfClass "/Game/BluePrint/oscillograph_Single_mode2_Blueprint.oscillograph_Single_mode2_Blueprint_C"))
      (Rendering|Material|SetMaterial (Variables|/Script/Engine.StaticMeshActor|GetStaticMeshComponent _returnvalue) 0 "/Game/Oscil/Meshes/Materials/Glow_LED_Inst.Glow_LED_Inst")
      (bind _returnvalue_2 (Actor|GetActorOfClass "/Game/BluePrint/CH1_Blueprint.CH1_Blueprint_C"))
      (Rendering|Material|SetMaterial (Variables|/Script/Engine.StaticMeshActor|GetStaticMeshComponent _returnvalue_2) 0 "/Game/Oscil/Meshes/Materials/Glow_CH1_Inst.Glow_CH1_Inst")
      (bind _returnvalue_3 (Actor|GetActorOfClass "/Game/ImageStreaming/BP_Image_Streaming.BP_Image_Streaming_C"))
      (Default|OnOff _returnvalue_3))
    (:B
      (Rendering|Material|SetMaterial _staticmeshcomponent 0 "/Game/Oscil/Meshes/Materials/Material_001.Material_001")
      (Utilities|FlowControl|Sequence
        (:then_0
          (bind _returnvalue_4 (Actor|GetActorOfClass "/Game/BluePrint/oscillograph_Single_mode2_Blueprint.oscillograph_Single_mode2_Blueprint_C"))
          (Rendering|Material|SetMaterial (Variables|/Script/Engine.StaticMeshActor|GetStaticMeshComponent _returnvalue_4) 0 "/Game/Oscil/Meshes/Materials/Material_leds.Material_leds"))
        (:then_1
          (bind _returnvalue_5 (Actor|GetActorOfClass "/Game/BluePrint/oscillograph_Normal2_Blueprint.oscillograph_Normal2_Blueprint_C"))
          (Rendering|Material|SetMaterial (Variables|/Script/Engine.StaticMeshActor|GetStaticMeshComponent _returnvalue_5) 0 "/Game/Oscil/Meshes/Materials/Material_leds.Material_leds"))
        (:then_2
          (bind _returnvalue_6 (Actor|GetActorOfClass "/Game/BluePrint/oscillograph_Auto_mode2_Blueprint.oscillograph_Auto_mode2_Blueprint_C"))
          (Rendering|Material|SetMaterial (Variables|/Script/Engine.StaticMeshActor|GetStaticMeshComponent _returnvalue_6) 0 "/Game/Oscil/Meshes/Materials/Material_leds.Material_leds"))
        (:then_3
          (bind _returnvalue_7 (Actor|GetActorOfClass "/Game/BluePrint/Screen_menu_Blueprint.Screen_menu_Blueprint_C"))
          (Rendering|Material|SetMaterial (Variables|/Script/Engine.StaticMeshActor|GetStaticMeshComponent _returnvalue_7) 0 "/Game/Oscil/OscScreen/WORKED/Materials/Clear_screen.Clear_screen"))
        (:then_4
          (bind _returnvalue_8 (Actor|GetActorOfClass "/Game/BluePrint/CH1_Blueprint.CH1_Blueprint_C"))
          (Rendering|Material|SetMaterial (Variables|/Script/Engine.StaticMeshActor|GetStaticMeshComponent _returnvalue_8) 0 "/Game/Oscil/Meshes/Materials/Glow_CH1.Glow_CH1"))
        (:then_5
          (bind _returnvalue_9 (Actor|GetActorOfClass "/Game/BluePrint/CH2_Blueprint.CH2_Blueprint_C"))
          (Rendering|Material|SetMaterial (Variables|/Script/Engine.StaticMeshActor|GetStaticMeshComponent _returnvalue_9) 0 "/Game/Oscil/Meshes/Materials/Glow_CH2.Glow_CH2"))
        (:then_6
          (bind _returnvalue_10 (Actor|GetActorOfClass "/Game/BluePrint/CH3_Blueprint.CH3_Blueprint_C"))
          (Rendering|Material|SetMaterial (Variables|/Script/Engine.StaticMeshActor|GetStaticMeshComponent _returnvalue_10) 0 "/Game/Oscil/Meshes/Materials/Glow_CH3.Glow_CH3"))
        (:then_7
          (bind _returnvalue_11 (Actor|GetActorOfClass "/Game/BluePrint/CH4_Blueprint.CH4_Blueprint_C"))
          (Rendering|Material|SetMaterial (Variables|/Script/Engine.StaticMeshActor|GetStaticMeshComponent _returnvalue_11) 0 "/Game/Oscil/Meshes/Materials/Glow_CH4.Glow_CH4"))
        (:then_8
          (bind _returnvalue_12 (Actor|GetActorOfClass "/Game/ImageStreaming/BP_Image_Streaming.BP_Image_Streaming_C"))
          (Default|OnOff _returnvalue_12))
        (:then_9
          (bind _returnvalue_13 (Actor|GetActorOfClass "/Game/BluePrint/oscillograph_Run_Stop2_Blueprint.oscillograph_Run_Stop2_Blueprint_C"))
          (Rendering|Material|SetMaterial (Variables|/Script/Engine.StaticMeshActor|GetStaticMeshComponent _returnvalue_13) 0 "/Game/Oscil/Meshes/Materials/Material_039.Material_039"))))))

(event EventTick
  (params (DeltaSeconds :type Float%20%28single-precision%29))
  (Utilities|FlowControl|Delay 5.0)
  (bind _returnvalue (Actor|GetActorOfClass "/Game/ImageStreaming/BP_Image_Streaming.BP_Image_Streaming_C"))
  (if (Variables|/Game/ImageStreaming/BP_Image_Streaming.BP_Image_Streaming_C|GetStatus _returnvalue)
    (bind _returnvalue_2 (Actor|GetActorOfClass "/Game/BluePrint/oscillograph_Run_Stop2_Blueprint.oscillograph_Run_Stop2_Blueprint_C"))
    (Utilities|FlowControl|FlipFlop
      (:A
        (Rendering|Material|SetMaterial (Variables|/Script/Engine.StaticMeshActor|GetStaticMeshComponent _returnvalue_2) 0 "/Game/Oscil/Meshes/Materials/Glow_RUN_Inst.Glow_RUN_Inst"))
      (:B
        (Rendering|Material|SetMaterial (Variables|/Script/Engine.StaticMeshActor|GetStaticMeshComponent _returnvalue_2) 0 "/Game/Oscil/Meshes/Materials/Glow_RUN.Glow_RUN")))))

(fn ConstructionScript)