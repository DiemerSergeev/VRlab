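; Right-side oscilloscope menu button that, when grabbed, flips the page on the screen menu.
; It checks each menu Blueprint's Status, then swaps the screen material and updates page state: Storage, manual Cursor and Ref toggle two pages, Utility and Math cycle three.
; Cursor mode events set CursorState, screen material and reset the page.
; Storage and Ref write their page to the Cursor Blueprint; other menu branches are empty.
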(event OnGrabbed(GrabComponent)
  (Utilities|FlowControl|Sequence
    (:then_0
      (bind _returnvalue (Actor|GetActorOfClass "/Game/BluePrint/oscillograph_Measure2_Blueprint.oscillograph_Measure2_Blueprint_C"))
      (if (Variables|/Game/BluePrint/oscillograph_Measure2_Blueprint.oscillograph_Measure2_Blueprint_C|GetStatus _returnvalue)
        _))
    (:then_1
      (bind _returnvalue_2 (Actor|GetActorOfClass "/Game/BluePrint/oscillograph_Storage2_Blueprint.oscillograph_Storage2_Blueprint_C"))
      (if (Variables|/Game/BluePrint/oscillograph_Storage2_Blueprint.oscillograph_Storage2_Blueprint_C|GetStatus _returnvalue_2)
        (if (== (Variables|/Game/BluePrint/oscillograph_Storage2_Blueprint.oscillograph_Storage2_Blueprint_C|GetStatus%20sheet _returnvalue_2) 1)
          (bind _returnvalue_3 (Actor|GetActorOfClass "/Game/BluePrint/Screen_menu_Blueprint.Screen_menu_Blueprint_C"))
          (Rendering|Material|SetMaterial (Variables|/Script/Engine.StaticMeshActor|GetStaticMeshComponent _returnvalue_3) 0 "/Game/Oscil/OscScreen/WORKED/Materials/storage2_Mat.storage2_Mat")
          (bind _returnvalue_4 (Actor|GetActorOfClass "/Game/BluePrint/oscillograph_Cursor2_Blueprint.oscillograph_Cursor2_Blueprint_C"))
          (Variables|/Game/BluePrint/oscillograph_Cursor2_Blueprint.oscillograph_Cursor2_Blueprint_C|SetStatus_sheet _returnvalue_4 2)
          (elif (== (Variables|/Game/BluePrint/oscillograph_Storage2_Blueprint.oscillograph_Storage2_Blueprint_C|GetStatus%20sheet _returnvalue_2) 2)
            (bind _returnvalue_5 (Actor|GetActorOfClass "/Game/BluePrint/Screen_menu_Blueprint.Screen_menu_Blueprint_C"))
            (Rendering|Material|SetMaterial (Variables|/Script/Engine.StaticMeshActor|GetStaticMeshComponent _returnvalue_5) 0 "/Game/Oscil/OscScreen/WORKED/Materials/storage1_Mat.storage1_Mat")
            (bind _returnvalue_6 (Actor|GetActorOfClass "/Game/BluePrint/oscillograph_Cursor2_Blueprint.oscillograph_Cursor2_Blueprint_C"))
            (Variables|/Game/BluePrint/oscillograph_Cursor2_Blueprint.oscillograph_Cursor2_Blueprint_C|SetStatus_sheet _returnvalue_6 1)))))
    (:then_2
      (bind _returnvalue_7 (Actor|GetActorOfClass "/Game/BluePrint/oscillograph_Cursor2_Blueprint.oscillograph_Cursor2_Blueprint_C"))
      (if (Variables|/Game/BluePrint/oscillograph_Cursor2_Blueprint.oscillograph_Cursor2_Blueprint_C|GetStatus _returnvalue_7)
        (if (== (Variables|Default|GetCursor%20state) 0)
          (if (== (Variables|/Game/BluePrint/oscillograph_Cursor2_Blueprint.oscillograph_Cursor2_Blueprint_C|GetStatus_sheet _returnvalue_7) 1)
            (bind _returnvalue_8 (Actor|GetActorOfClass "/Game/BluePrint/Screen_menu_Blueprint.Screen_menu_Blueprint_C"))
            (Rendering|Material|SetMaterial (Variables|/Script/Engine.StaticMeshActor|GetStaticMeshComponent _returnvalue_8) 0 "/Game/Oscil/OscScreen/WORKED/Materials/cursor_manual_2_Mat.cursor_manual_2_Mat")
            (bind _returnvalue_9 (Actor|GetActorOfClass "/Game/BluePrint/oscillograph_Cursor2_Blueprint.oscillograph_Cursor2_Blueprint_C"))
            (Variables|/Game/BluePrint/oscillograph_Cursor2_Blueprint.oscillograph_Cursor2_Blueprint_C|SetStatus_sheet _returnvalue_9 2)
            (elif (== (Variables|/Game/BluePrint/oscillograph_Cursor2_Blueprint.oscillograph_Cursor2_Blueprint_C|GetStatus_sheet _returnvalue_7) 2)
              (bind _returnvalue_10 (Actor|GetActorOfClass "/Game/BluePrint/Screen_menu_Blueprint.Screen_menu_Blueprint_C"))
              (Rendering|Material|SetMaterial (Variables|/Script/Engine.StaticMeshActor|GetStaticMeshComponent _returnvalue_10) 0 "/Game/Oscil/OscScreen/WORKED/Materials/cursor_manual_1_Mat.cursor_manual_1_Mat")
              (bind _returnvalue_11 (Actor|GetActorOfClass "/Game/BluePrint/oscillograph_Cursor2_Blueprint.oscillograph_Cursor2_Blueprint_C"))
              (Variables|/Game/BluePrint/oscillograph_Cursor2_Blueprint.oscillograph_Cursor2_Blueprint_C|SetStatus_sheet _returnvalue_11 1))))))
    (:then_3
      (bind _returnvalue_12 (Actor|GetActorOfClass "/Game/BluePrint/oscillograph_Display2_Blueprint.oscillograph_Display2_Blueprint_C"))
      (if (Variables|/Game/BluePrint/oscillograph_Display2_Blueprint.oscillograph_Display2_Blueprint_C|GetStatus _returnvalue_12)
        _))
    (:then_4
      (bind _returnvalue_13 (Actor|GetActorOfClass "/Game/BluePrint/oscillograph_Utility2_Blueprint.oscillograph_Utility2_Blueprint_C"))
      (if (Variables|/Game/BluePrint/oscillograph_Utility2_Blueprint.oscillograph_Utility2_Blueprint_C|GetStatus _returnvalue_13)
        (if (== (Variables|/Game/BluePrint/oscillograph_Utility2_Blueprint.oscillograph_Utility2_Blueprint_C|GetStatusSheetR _returnvalue_13) 1)
          (bind _returnvalue_14 (Actor|GetActorOfClass "/Game/BluePrint/Screen_menu_Blueprint.Screen_menu_Blueprint_C"))
          (Rendering|Material|SetMaterial (Variables|/Script/Engine.StaticMeshActor|GetStaticMeshComponent _returnvalue_14) 0 "/Game/Oscil/OscScreen/WORKED/Materials/utility_3_Mat.utility_3_Mat")
          (bind _returnvalue_15 (Actor|GetActorOfClass "/Game/BluePrint/oscillograph_Utility2_Blueprint.oscillograph_Utility2_Blueprint_C"))
          (Variables|/Game/BluePrint/oscillograph_Utility2_Blueprint.oscillograph_Utility2_Blueprint_C|SetStatusSheetR _returnvalue_15 3)
          (elif (== (Variables|/Game/BluePrint/oscillograph_Utility2_Blueprint.oscillograph_Utility2_Blueprint_C|GetStatusSheetR _returnvalue_13) 2)
            (bind _returnvalue_16 (Actor|GetActorOfClass "/Game/BluePrint/Screen_menu_Blueprint.Screen_menu_Blueprint_C"))
            (Rendering|Material|SetMaterial (Variables|/Script/Engine.StaticMeshActor|GetStaticMeshComponent _returnvalue_16) 0 "/Game/Oscil/OscScreen/WORKED/Materials/utility_1_Mat.utility_1_Mat")
            (bind _returnvalue_17 (Actor|GetActorOfClass "/Game/BluePrint/oscillograph_Utility2_Blueprint.oscillograph_Utility2_Blueprint_C"))
            (Variables|/Game/BluePrint/oscillograph_Utility2_Blueprint.oscillograph_Utility2_Blueprint_C|SetStatusSheetR _returnvalue_17 1)
            (elif (== (Variables|/Game/BluePrint/oscillograph_Utility2_Blueprint.oscillograph_Utility2_Blueprint_C|GetStatusSheetR _returnvalue_13) 3)
              (bind _returnvalue_18 (Actor|GetActorOfClass "/Game/BluePrint/Screen_menu_Blueprint.Screen_menu_Blueprint_C"))
              (Rendering|Material|SetMaterial (Variables|/Script/Engine.StaticMeshActor|GetStaticMeshComponent _returnvalue_18) 0 "/Game/Oscil/OscScreen/WORKED/Materials/utility_2_Mat.utility_2_Mat")
              (bind _returnvalue_19 (Actor|GetActorOfClass "/Game/BluePrint/oscillograph_Utility2_Blueprint.oscillograph_Utility2_Blueprint_C"))
              (Variables|/Game/BluePrint/oscillograph_Utility2_Blueprint.oscillograph_Utility2_Blueprint_C|SetStatusSheetR _returnvalue_19 2))))))
    (:then_5
      (bind _returnvalue_20 (Actor|GetActorOfClass "/Game/BluePrint/oscillograph_Math2_Blueprint.oscillograph_Math2_Blueprint_C"))
      (if (Variables|/Game/BluePrint/oscillograph_Math2_Blueprint.oscillograph_Math2_Blueprint_C|GetStatus _returnvalue_20)
        (if (== (Variables|/Game/BluePrint/oscillograph_Math2_Blueprint.oscillograph_Math2_Blueprint_C|GetStatus_sheet_R _returnvalue_20) 1)
          (bind _returnvalue_21 (Actor|GetActorOfClass "/Game/BluePrint/Screen_menu_Blueprint.Screen_menu_Blueprint_C"))
          (Rendering|Material|SetMaterial (Variables|/Script/Engine.StaticMeshActor|GetStaticMeshComponent _returnvalue_21) 0 "/Game/Oscil/OscScreen/WORKED/Materials/MATH_3_X_Mat.MATH_3_X_Mat")
          (bind _returnvalue_22 (Actor|GetActorOfClass "/Game/BluePrint/oscillograph_Math2_Blueprint.oscillograph_Math2_Blueprint_C"))
          (Variables|/Game/BluePrint/oscillograph_Math2_Blueprint.oscillograph_Math2_Blueprint_C|SetStatus_sheet_R _returnvalue_22 3)
          (elif (== (Variables|/Game/BluePrint/oscillograph_Math2_Blueprint.oscillograph_Math2_Blueprint_C|GetStatus_sheet_R _returnvalue_20) 2)
            (bind _returnvalue_23 (Actor|GetActorOfClass "/Game/BluePrint/Screen_menu_Blueprint.Screen_menu_Blueprint_C"))
            (Rendering|Material|SetMaterial (Variables|/Script/Engine.StaticMeshActor|GetStaticMeshComponent _returnvalue_23) 0 "/Game/Oscil/OscScreen/WORKED/Materials/MATH_1_X_Mat.MATH_1_X_Mat")
            (bind _returnvalue_24 (Actor|GetActorOfClass "/Game/BluePrint/oscillograph_Math2_Blueprint.oscillograph_Math2_Blueprint_C"))
            (Variables|/Game/BluePrint/oscillograph_Math2_Blueprint.oscillograph_Math2_Blueprint_C|SetStatus_sheet_R _returnvalue_24 1)
            (elif (== (Variables|/Game/BluePrint/oscillograph_Math2_Blueprint.oscillograph_Math2_Blueprint_C|GetStatus_sheet_R _returnvalue_20) 3)
              (bind _returnvalue_25 (Actor|GetActorOfClass "/Game/BluePrint/Screen_menu_Blueprint.Screen_menu_Blueprint_C"))
              (Rendering|Material|SetMaterial (Variables|/Script/Engine.StaticMeshActor|GetStaticMeshComponent _returnvalue_25) 0 "/Game/Oscil/OscScreen/WORKED/Materials/MATH_2_X_Mat.MATH_2_X_Mat")
              (bind _returnvalue_26 (Actor|GetActorOfClass "/Game/BluePrint/oscillograph_Math2_Blueprint.oscillograph_Math2_Blueprint_C"))
              (Variables|/Game/BluePrint/oscillograph_Math2_Blueprint.oscillograph_Math2_Blueprint_C|SetStatus_sheet_R _returnvalue_26 2))))))
    (:then_6
      (bind _returnvalue_27 (Actor|GetActorOfClass "/Game/BluePrint/oscillograph_Ref2_Blueprint.oscillograph_Ref2_Blueprint_C"))
      (if (Variables|/Game/BluePrint/oscillograph_Ref2_Blueprint.oscillograph_Ref2_Blueprint_C|GetStatus _returnvalue_27)
        (if (== (Variables|/Game/BluePrint/oscillograph_Ref2_Blueprint.oscillograph_Ref2_Blueprint_C|GetStatus%20sheet _returnvalue_27) 1)
          (bind _returnvalue_28 (Actor|GetActorOfClass "/Game/BluePrint/Screen_menu_Blueprint.Screen_menu_Blueprint_C"))
          (Rendering|Material|SetMaterial (Variables|/Script/Engine.StaticMeshActor|GetStaticMeshComponent _returnvalue_28) 0 "/Game/Oscil/OscScreen/WORKED/Materials/ref2_Mat.ref2_Mat")
          (bind _returnvalue_29 (Actor|GetActorOfClass "/Game/BluePrint/oscillograph_Cursor2_Blueprint.oscillograph_Cursor2_Blueprint_C"))
          (Variables|/Game/BluePrint/oscillograph_Cursor2_Blueprint.oscillograph_Cursor2_Blueprint_C|SetStatus_sheet _returnvalue_29 2)
          (elif (== (Variables|/Game/BluePrint/oscillograph_Ref2_Blueprint.oscillograph_Ref2_Blueprint_C|GetStatus%20sheet _returnvalue_27) 2)
            (bind _returnvalue_30 (Actor|GetActorOfClass "/Game/BluePrint/Screen_menu_Blueprint.Screen_menu_Blueprint_C"))
            (Rendering|Material|SetMaterial (Variables|/Script/Engine.StaticMeshActor|GetStaticMeshComponent _returnvalue_30) 0 "/Game/Oscil/OscScreen/WORKED/Materials/ref1_Mat.ref1_Mat")
            (bind _returnvalue_31 (Actor|GetActorOfClass "/Game/BluePrint/oscillograph_Cursor2_Blueprint.oscillograph_Cursor2_Blueprint_C"))
            (Variables|/Game/BluePrint/oscillograph_Cursor2_Blueprint.oscillograph_Cursor2_Blueprint_C|SetStatus_sheet _returnvalue_31 1)))))
    (:then_7
      (bind _returnvalue_32 (Actor|GetActorOfClass "/Game/BluePrint/oscillograph_Force2_Blueprint.oscillograph_Force2_Blueprint_C"))
      (if (Variables|/Game/BluePrint/oscillograph_Force2_Blueprint.oscillograph_Force2_Blueprint_C|GetStatus _returnvalue_32)
        _))
    (:then_8
      (bind _returnvalue_33 (Actor|GetActorOfClass "/Game/BluePrint/oscillograph_Help2_Blueprint.oscillograph_Help2_Blueprint_C"))
      (if (Variables|/Game/BluePrint/oscillograph_Help2_Blueprint.oscillograph_Help2_Blueprint_C|GetStatus _returnvalue_33)
        _))
    (:then_9
      (bind _returnvalue_34 (Actor|GetActorOfClass "/Game/BluePrint/oscillograph_S2_Blueprint.oscillograph_S2_Blueprint_C"))
      (if (Variables|/Game/BluePrint/oscillograph_S2_Blueprint.oscillograph_S2_Blueprint_C|GetStatus _returnvalue_34)
        _))
    (:then_10
      (bind _returnvalue_35 (Actor|GetActorOfClass "/Game/BluePrint/oscillograph_Menu4_Blueprint.oscillograph_Menu4_Blueprint_C"))
      (if (Variables|/Game/BluePrint/oscillograph_Menu4_Blueprint.oscillograph_Menu4_Blueprint_C|GetStatus _returnvalue_35)
        _))
    (:then_11
      (bind _returnvalue_36 (Actor|GetActorOfClass "/Game/BluePrint/oscillograph_Menu3_Blueprint.oscillograph_Menu3_Blueprint_C"))
      (if (Variables|/Game/BluePrint/oscillograph_Menu3_Blueprint.oscillograph_Menu3_Blueprint_C|GetStatus _returnvalue_36)
        _))
    (:then_12
      (bind _returnvalue_37 (Actor|GetActorOfClass "/Game/BluePrint/oscillograph_Acquire2_Blueprint.oscillograph_Acquire2_Blueprint_C"))
      (if (Variables|/Game/BluePrint/oscillograph_Acquire2_Blueprint.oscillograph_Acquire2_Blueprint_C|GetStatus _returnvalue_37)
        _))))

(event Custom|Cursor%20off
  (Variables|Default|SetCursor%20state 1)
  (bind _returnvalue (Actor|GetActorOfClass "/Game/BluePrint/Screen_menu_Blueprint.Screen_menu_Blueprint_C"))
  (Rendering|Material|SetMaterial (Variables|/Script/Engine.StaticMeshActor|GetStaticMeshComponent _returnvalue) 0 "/Game/Oscil/OscScreen/WORKED/Materials/Menu1_Mat.Menu1_Mat")
  (bind _returnvalue_2 (Actor|GetActorOfClass "/Game/BluePrint/oscillograph_Cursor2_Blueprint.oscillograph_Cursor2_Blueprint_C"))
  (Variables|/Game/BluePrint/oscillograph_Cursor2_Blueprint.oscillograph_Cursor2_Blueprint_C|SetStatus_sheet _returnvalue_2 1))

(event Custom|Cursor%20manual
  (Variables|Default|SetCursor%20state 0)
  (bind _returnvalue (Actor|GetActorOfClass "/Game/BluePrint/Screen_menu_Blueprint.Screen_menu_Blueprint_C"))
  (Rendering|Material|SetMaterial (Variables|/Script/Engine.StaticMeshActor|GetStaticMeshComponent _returnvalue) 0 "/Game/Oscil/OscScreen/WORKED/Materials/cursor_manual_1_Mat.cursor_manual_1_Mat")
  (bind _returnvalue_2 (Actor|GetActorOfClass "/Game/BluePrint/oscillograph_Cursor2_Blueprint.oscillograph_Cursor2_Blueprint_C"))
  (Variables|/Game/BluePrint/oscillograph_Cursor2_Blueprint.oscillograph_Cursor2_Blueprint_C|SetStatus_sheet _returnvalue_2 1))

(event Custom|Cursor%20auto
  (Variables|Default|SetCursor%20state 2)
  (bind _returnvalue (Actor|GetActorOfClass "/Game/BluePrint/Screen_menu_Blueprint.Screen_menu_Blueprint_C"))
  (Rendering|Material|SetMaterial (Variables|/Script/Engine.StaticMeshActor|GetStaticMeshComponent _returnvalue) 0 "/Game/Oscil/OscScreen/WORKED/Materials/cursor_auto_Mat.cursor_auto_Mat")
  (bind _returnvalue_2 (Actor|GetActorOfClass "/Game/BluePrint/oscillograph_Cursor2_Blueprint.oscillograph_Cursor2_Blueprint_C"))
  (Variables|/Game/BluePrint/oscillograph_Cursor2_Blueprint.oscillograph_Cursor2_Blueprint_C|SetStatus_sheet _returnvalue_2 1))

(event Custom|Cursor%20track
  (Variables|Default|SetCursor%20state 3)
  (bind _returnvalue (Actor|GetActorOfClass "/Game/BluePrint/Screen_menu_Blueprint.Screen_menu_Blueprint_C"))
  (Rendering|Material|SetMaterial (Variables|/Script/Engine.StaticMeshActor|GetStaticMeshComponent _returnvalue) 0 "/Game/Oscil/OscScreen/WORKED/Materials/cursor_track_Mat.cursor_track_Mat")
  (bind _returnvalue_2 (Actor|GetActorOfClass "/Game/BluePrint/oscillograph_Cursor2_Blueprint.oscillograph_Cursor2_Blueprint_C"))
  (Variables|/Game/BluePrint/oscillograph_Cursor2_Blueprint.oscillograph_Cursor2_Blueprint_C|SetStatus_sheet _returnvalue_2 1))

(fn ConstructionScript)